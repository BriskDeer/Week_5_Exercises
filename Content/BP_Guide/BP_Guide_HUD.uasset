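; HUD for the guide game that draws score, time and player level on screen, plus a game-over screen with rank and a "Press Enter" prompt.
; BeginPlay casts the game mode to BP_Guide_GameMode and caches it.
; DrawHUD reads that game mode every frame and renders colored canvas text at fixed screen positions, adding the game-over lines while its GameOver flag is set.
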(event EventBeginPlay
  (bind _asbp_guide_game_mode (Utilities|Casting|CastToBP_Guide_GameMode (Game|GetGameMode)))
  (Variables|Default|SetMy_Guide_GameMode _asbp_guide_game_mode))

(event Collision|EventActorBeginOverlap
  (params (OtherActor :type Actor%20Object%20Reference)))

(event EventTick
  (params (DeltaSeconds :type Float%20%28single-precision%29)))

(event EventDrawHUD
  (params (SizeX :type Integer) (SizeY :type Integer))
  (HUD|DrawText (Utilities|String|BuildString(Integer) "Score: " "" (Variables|/Game/BP_Guide/BP_Guide_GameMode.BP_Guide_GameMode_C|GetScore (Variables|Default|GetMy_Guide_GameMode))) "(R=0.567708,G=0.544920,B=0.002957,A=1.000000)" 1e+01 1e+01 0 3.0 false)
  (HUD|DrawText (Utilities|String|BuildString(Integer) "Time: " "" (Variables|/Game/BP_Guide/BP_Guide_GameMode.BP_Guide_GameMode_C|GetTime (Variables|Default|GetMy_Guide_GameMode))) "(R=0.557292,G=0.034831,B=0.034831,A=1.000000)" 3e+02 1e+01 0 3.0 false)
  (HUD|DrawText (Utilities|String|BuildString(Integer) "Player Level: " "" (Variables|/Game/BP_Guide/BP_Guide_GameMode.BP_Guide_GameMode_C|GetLevel (Variables|Default|GetMy_Guide_GameMode))) "(R=0.025624,G=0.039868,B=0.557292,A=1.000000)" 5.5e+02 1e+01 0 3.0 false)
  (if (Variables|/Game/BP_Guide/BP_Guide_GameMode.BP_Guide_GameMode_C|GetGameOver (Variables|Default|GetMy_Guide_GameMode))
    (HUD|DrawText "GAME OVER" "(R=0.557292,G=0.055960,B=0.028229,A=1.000000)" 4e+02 2e+02 0 3.0 false)
    (HUD|DrawText "Press Enter" "(R=0.557292,G=0.023221,B=0.023221,A=1.000000)" 4e+02 4e+02 0 3.0 false)
    (HUD|DrawText (Utilities|String|Append "Rank:" (Variables|/Game/BP_Guide/BP_Guide_GameMode.BP_Guide_GameMode_C|GetRank (Variables|Default|GetMy_Guide_GameMode))) "(R=1.000000,G=0.000000,B=0.000000,A=1.000000)" 4e+02 3e+02 0 3.0 false)))

(fn ConstructionScript)